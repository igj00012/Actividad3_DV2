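; Enemy Blueprint that wanders the level and chases the player when it spots a pawn.
; It loops AI Move To toward random reachable points, pausing between successful moves.
; Pawn Sensing clears CanAttack and starts a move toward player 0, setting the flag again on reaching attack range.
; A retriggerable delay, refreshed by each sighting, returns it to wandering one second after sight is lost.
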(event OnSeePawn(PawnSensing)
  (params (Pawn :type Pawn%20Object%20Reference))
  ;[0.15 0.15 0.15 0.5] Cuando ve al jugador lo persigue
  (Utilities|IsValid Pawn
    (:Is%20Valid
      (Variables|Default|SetCanAttack false)
      (Utilities|FlowControl|Sequence
        (:then_0
          (AI|AIMoveTo self "0, 0, 0" (Game|Player|GetPlayerPawn 0) (Variables|Default|GetAttackRange) false
            (:OnSuccess
              (Variables|Default|SetCanAttack true))))
        (:then_1
          ;;[0.15 0.15 0.15 0.5] Si deja de verlo durante un segundo vuelve a su comportamiento aleatorio
          (Utilities|FlowControl|RetriggerableDelay 1.0)
          (CallFunction|MovetoRandomPoint))))))

(event Custom|MoveToRandomPoint
  ;[0.15 0.15 0.15 0.5] Movimiento aleatorio por el escenario
  (AI|AIMoveTo self (.RandomLocation (AI|Navigation|GetRandomReachablePointinRadius (Transformation|GetActorLocation) 2e+03 0 0)) 0 5.0 false
    (:OnSuccess
      (Utilities|FlowControl|Delay (Variables|Default|GetDelayBetweenPoints))
      (CallFunction|MovetoRandomPoint))))

(event EventBeginPlay
  (CallFunction|MovetoRandomPoint))

(fn ConstructionScript)