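; BP_WizardEnemy is a ranged wizard enemy that closes on its target and attacks with fireballs.
; A looping timer set on BeginPlay runs AIAttack, which moves the wizard into attack range and then starts an attack if none is active.
; StartAttack and EndAttack toggle the attacking flag and lock or restore walking movement.
; A separate Attack event spawns a fireball at a mesh socket, passing it the target and damage.
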(event Custom|StartAttack
  ;[0.15 0.15 0.15 0.5] Control de la animación de ataque
  (Variables|Default|SetIsAttacking true)
  (Pawn|Components|CharacterMovement|DisableMovement (Variables|Character|GetCharacterMovement)))

(event Custom|Attack
  ;[0.15 0.15 0.15 0.5] Lógica del ataque
  (bind _returnvalue (Game|SpawnActorfromClass "/Game/Enemies/BP_FireBall.BP_FireBall_C" (Transformation|GetSocketTransform (Variables|Character|GetMesh) "MagicSpawnPoint" "RTS_World") "Undefined" "MultiplyWithRoot" 0 (Variables|Default|GetTarget) 0))
  (Utilities|IsValid _returnvalue
    (:Is%20Valid
      (Variables|/Game/Enemies/BP_FireBall.BP_FireBall_C|SetDamage _returnvalue (Variables|Default|GetDamage)))))

(event Custom|EndAttack
  ;[0.15 0.15 0.15 0.5] Control de la animación de ataque
  (Variables|Default|SetIsAttacking false)
  (Pawn|Components|CharacterMovement|SetMovementMode (Variables|Character|GetCharacterMovement) "MOVE_Walking" 0))

(event Custom|AIAttack
  (bind _target (Variables|Default|GetTarget))
  (Utilities|IsValid _target
    (:Is%20Valid
      (if (> (Transformation|GetDistanceTo _target) (Variables|Default|GetAttackRange))
        (AI|AIMoveTo self "0, 0, 0" (Variables|Default|GetTarget) (Variables|Default|GetAttackRange) false
          (:OnSuccess
            (if (not (Variables|Default|GetIsAttacking))
              (CallFunction|StartAttack))))
        (elif (not (Variables|Default|GetIsAttacking))
          (CallFunction|StartAttack))))))

(event EventBeginPlay
  (|CallParentFunction)
  (bind _output_get (Variables|Default|SetAttackDelay 2.5))
  (Utilities|Time|SetTimerbyEvent (delegate Custom|AIAttack) _output_get true))

(fn ConstructionScript
  (|CallParentFunction))