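; BP_FireBall is an enemy fireball projectile that homes in on the player and damages them on contact.
; Each tick it moves toward player pawn 0 along the unnormalized offset scaled by Speed, so it slows as it closes in, without sweeping.
; Sphere overlap with BP_ThirdPersonCharacter calls UpdateHealth with Damage and destroys the fireball after a short delay.
; Other overlaps destroy it immediately, and LifeSpan limits its lifetime.
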(event OnComponentBeginOverlap(Sphere)
  (params (OverlappedComponent :type Primitive%20Component%20Object%20Reference) (OtherActor :type Actor%20Object%20Reference) (OtherComp :type Primitive%20Component%20Object%20Reference) (OtherBodyIndex :type Integer) (bFromSweep :type Boolean) (SweepResult :type Hit%20Result%20Structure%20%28by%20ref%29))
  ;[0.15 0.15 0.15 0.5] Lógica del daño de la bala
  (bind _asbp_third_person_character (Utilities|Casting|CastToBP_ThirdPersonCharacter OtherActor)
    (:then
      (Utilities|IsValid _asbp_third_person_character
        (:Is%20Valid
          (Default|UpdateHealth _asbp_third_person_character (Variables|Default|GetDamage))
          (Utilities|FlowControl|Delay 0.2))))
    (:CastFailed
      _))
  (Actor|DestroyActor))

(event EventTick
  (params (DeltaSeconds :type Float%20%28single-precision%29))
  ;[0.15 0.15 0.15 0.5] Movimiento de la bala hacia el jugador
  (Transformation|SetActorLocation (+ (* (* DeltaSeconds (Variables|Default|GetSpeed)) (- (Transformation|GetActorLocation (Game|Player|GetPlayerPawn 0)) (Transformation|GetActorLocation))) (Transformation|GetActorLocation)) false false))

(event EventBeginPlay
  ;[0.15 0.15 0.15 0.5] Se destruye tras x segundos
  (Actor|SetLifeSpan (Variables|Default|GetLifeSpan)))

(fn ConstructionScript)